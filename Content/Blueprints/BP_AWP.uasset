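; BP_AWP is a sniper weapon Blueprint that adds a scope overlay and zoom when the player targets.
; It creates the WBP_SniperHUD widget on BeginPlay, then on StartTarget shows it and narrows the TargetingFOV on player 0's ShooterPlayerCameraManager.
; EndTarget, OnUnEquip and Destroyed share one cleanup path that removes the overlay and sets a wider TargetingFOV.
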(event EventBeginPlay
  (bind _returnvalue (UserInterface|CreateWidget "/Game/UI/WBP_SniperHUD.WBP_SniperHUD_C"))
  (Variables|Default|SetSniperHUD _returnvalue))

(event EventDestroyed
  (bind _sniperhud (Variables|Default|GetSniperHUD))
  (Utilities|IsValid _sniperhud
    (:Is%20Valid
      (Widget|RemovefromParent _sniperhud)
      (bind _asshooter_player_camera_manager (Utilities|Casting|CastToShooterPlayerCameraManager (Variables|/Script/Engine.PlayerController|GetPlayerCameraManager (Game|GetPlayerController 0))))
      (Variables|/Script/prototype.ShooterPlayerCameraManager|SetTargetingFOV _asshooter_player_camera_manager 65.0))))

(event EventOnUnEquip
  (bind _sniperhud (Variables|Default|GetSniperHUD))
  (Utilities|IsValid _sniperhud
    (:Is%20Valid
      (Widget|RemovefromParent _sniperhud)
      (bind _asshooter_player_camera_manager (Utilities|Casting|CastToShooterPlayerCameraManager (Variables|/Script/Engine.PlayerController|GetPlayerCameraManager (Game|GetPlayerController 0))))
      (Variables|/Script/prototype.ShooterPlayerCameraManager|SetTargetingFOV _asshooter_player_camera_manager 65.0))))

(event EventStartTarget
  (bind _sniperhud (Variables|Default|GetSniperHUD))
  (Utilities|IsValid _sniperhud
    (:Is%20Valid
      (UserInterface|Viewport|AddtoViewport _sniperhud 0)
      (bind _asshooter_player_camera_manager (Utilities|Casting|CastToShooterPlayerCameraManager (Variables|/Script/Engine.PlayerController|GetPlayerCameraManager (Game|GetPlayerController 0))))
      (Variables|/Script/prototype.ShooterPlayerCameraManager|SetTargetingFOV _asshooter_player_camera_manager 15.0))))

(event EventEndTarget
  (bind _sniperhud (Variables|Default|GetSniperHUD))
  (Utilities|IsValid _sniperhud
    (:Is%20Valid
      (Widget|RemovefromParent _sniperhud)
      (bind _asshooter_player_camera_manager (Utilities|Casting|CastToShooterPlayerCameraManager (Variables|/Script/Engine.PlayerController|GetPlayerCameraManager (Game|GetPlayerController 0))))
      (Variables|/Script/prototype.ShooterPlayerCameraManager|SetTargetingFOV _asshooter_player_camera_manager 65.0))))

(fn ConstructionScript)