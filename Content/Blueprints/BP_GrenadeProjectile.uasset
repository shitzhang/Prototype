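; Grenade projectile Blueprint whose detonation logic is present but disconnected, so none of it runs in this graph.
; BeginPlay is empty, and an unwired chain waits briefly and calls Explode.
; A second unwired chain spawns an explosion effect, applies full radial damage credited to the instigator, fires the RadialForceComp impulse, draws a debug sphere and destroys the actor.
; Damage and debug sphere share the radial force component's radius.
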(event EventBeginPlay)

(fn ConstructionScript)