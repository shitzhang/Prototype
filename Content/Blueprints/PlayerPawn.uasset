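; Player character Blueprint that computes foot IK offsets from the ground and plays a jumping jacks montage on F.
; Each Tick, IKFootTrace line-traces down at each foot socket's XY from actor height, and the results are smoothed with FInterpTo.
; The trace compensates for crouching and actor scale, returning zero without a hit.
; The construction script derives trace distance from the scaled capsule, scales the hand radius and seeds hand offsets from sockets.
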(event EventTick
  (params (DeltaSeconds :type Float%20%28single-precision%29))
  ;[1 1 1] Update IK Offset
  (bind _ikoffset (CallFunction|IKFootTrace (Variables|Default|GetIKTraceDistance) (Variables|Default|GetIKRightFootSocket)))
  (Variables|Default|SetIKOffsetRightFoot (Math|Interpolation|FInterpTo (Variables|Default|GetIKOffsetRightFoot) _ikoffset DeltaSeconds (Variables|Default|GetIKInterpSpeed)))
  (bind _ikoffset_2 (CallFunction|IKFootTrace (Variables|Default|GetIKTraceDistance) (Variables|Default|GetIKLeftFootSocket)))
  (Variables|Default|SetIKOffsetLeftFoot (Math|Interpolation|FInterpTo (Variables|Default|GetIKOffsetLeftFoot) _ikoffset_2 DeltaSeconds (Variables|Default|GetIKInterpSpeed))))

(event Input|KeyboardEvents|F
  (params (Key :type Key%20Structure :default "None"))
  (:Pressed
    (if (not (Animation|Montage|MontageIsPlaying (Components|SkeletalMesh|GetAnimInstance (Variables|Character|GetMesh self)) "/Game/Animation/Punch_Anims/JumpingJacks_Montage.JumpingJacks_Montage"))
      (Animation|PlayAnimMontage "/Game/Animation/Punch_Anims/JumpingJacks_Montage.JumpingJacks_Montage" 1.0 "None"))))

(fn ConstructionScript
  (Variables|Default|SetScale (.Z (Math|Vector|BreakVector (.Scale (Math|Transform|BreakTransform (Transformation|GetActorTransform))))))
  (Variables|Default|SetIKTraceDistance (* (Variables|/Script/Engine.CapsuleComponent|GetCapsuleHalfHeight (Variables|Default|GetCapsuleComponent)) (Variables|Default|GetScale)))
  ;[1 1 1] Set initial Hand Offsets
  (Variables|Default|SetHandRadius (* (Variables|Default|GetHandRadius) (Variables|Default|GetScale)))
  (Variables|Default|SetIKOffsetRightHand (Transformation|GetSocketLocation (Variables|Character|GetMesh) "RightHandSocket"))
  (Variables|Default|SetIKOffsetLeftHand (Transformation|GetSocketLocation (Variables|Character|GetMesh) "LeftHandSocket")))

(fn IKFootTrace
  (params (TraceDistance :type Float%20%28single-precision%29) (Socket :type Name))
  (bind _returnvalue (Transformation|GetActorLocation))
  (bind _self self)
  (bind _mesh (Variables|Character|GetMesh))
  (bind _actorcrouchlocationoffset (Variables|Default|GetActorCrouchLocationOffset))
  (bind _scale (Variables|Default|GetScale))
  (bind _returnvalue_2 (Transformation|GetSocketLocation _mesh Socket))
  (bind _z (Math|Vector|BreakVector _returnvalue))
  (bind _returnvalue_3 (* _actorcrouchlocationoffset _scale))
  (bind _biscrouched (Variables|Default|GetbIsCrouched _self))
  (bind (_x _y) (Math|Vector|BreakVector _returnvalue_2))
  (bind _returnvalue_4 (+ _z _returnvalue_3))
  (bind _returnvalue_5 (Math|Float|SelectFloat _returnvalue_4 _z _biscrouched))
  (bind _returnvalue_6 (- _returnvalue_5 TraceDistance))
  (bind _returnvalue_7 (Math|Vector|MakeVector _x _y _returnvalue_6))
  (bind (_outhit _returnvalue_8) (Collision|LineTraceByChannel (Math|Vector|MakeVector _x _y _z) _returnvalue_7 "TraceTypeQuery1" true 0 "None"))
  (return (Math|Float|SelectFloat (/ (Math|Vector|VectorLength (- _returnvalue_7 (.Location (Collision|BreakHitResult _outhit)))) (Variables|Default|GetScale)) 0.0 _returnvalue_8)))